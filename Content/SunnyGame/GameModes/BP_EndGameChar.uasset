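; End-game character that presents the closing narrative and then returns the player to the main menu.
; On BeginPlay it adds the input mapping context, shows the narrative screen widget and switches to UI-only input with a visible cursor.
; Skip button clicks advance three text pages by binding each next event without unbinding earlier ones.
; The final click plays a fade-out widget, then opens MainMenu after a delay.
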(event `self.ReceiveBeginPlay`
  (`EnhancedInputSubsystemInterface.AddMappingContext` (pcsubsystem `EnhancedInputLocalPlayerSubsystem` (`GameplayStatics.GetPlayerController` 0)) "/Game/SunnyGame/Inputs/IMC_PlayerInputs.IMC_PlayerInputs" 0 (struct))
  (`self.End Narrative`))

(event `End Narrative`
  (bind _returnvalue (`GameplayStatics.GetPlayerController` 0))
  ; Add Narrative Widget
  (bind _returnvalue_2 (`|CreateWidget` "/Game/SunnyGame/Widgets/WBP_NarrativeScreen.WBP_NarrativeScreen_C" (`GameplayStatics.GetPlayerController` 0)))
  (bind _output_get (set `self.Narrative Screen REF` _returnvalue_2))
  (`UserWidget.AddToViewport` _output_get 0)
  ; Set controller to affect only UI
  (set `PlayerController.bShowMouseCursor` true _returnvalue)
  (`WidgetBlueprintLibrary.SetInputMode_UIOnlyEx` _returnvalue (`self.Narrative Screen REF`))
  ; Start Page 1
  (set `TextBlock.Text` (`|GetArrayItem` (`self.End Narrative Texts`)) (`/Game/SunnyGame/Widgets/WBP_NarrativeScreen.Text_Narrative` (`self.Narrative Screen REF`)))
  (add `Button.OnClicked` (`/Game/SunnyGame/Widgets/WBP_NarrativeScreen.B_Skip` (`self.Narrative Screen REF`)) (delegate `Page 2`)))

(event `Page 2`
  (set `TextBlock.Text` (`|GetArrayItem` (`self.End Narrative Texts`) 1) (`/Game/SunnyGame/Widgets/WBP_NarrativeScreen.Text_Narrative` (`self.Narrative Screen REF`)))
  (add `Button.OnClicked` (`/Game/SunnyGame/Widgets/WBP_NarrativeScreen.B_Skip` (`self.Narrative Screen REF`)) (delegate `Blank Slate`)))

(event `Blank Slate`
  (bind _narrative_screen_ref (`self.Narrative Screen REF`))
  (set `TextBlock.Text` (`|GetArrayItem` (`self.End Narrative Texts`) 2) (`/Game/SunnyGame/Widgets/WBP_NarrativeScreen.Text_Narrative` _narrative_screen_ref))
  (set `TextBlock.Text` "End Game" (`/Game/SunnyGame/Widgets/WBP_NarrativeScreen.Text_Label` _narrative_screen_ref))
  (add `Button.OnClicked` (`/Game/SunnyGame/Widgets/WBP_NarrativeScreen.B_Skip` (`self.Narrative Screen REF`)) (delegate `FadeOut`)))

(event `FadeOut`
  ; Open Main Menu
  (bind _returnvalue (`|CreateWidget` "/Game/SunnyGame/Widgets/WBP_Fade.WBP_Fade_C"))
  (`UserWidget.AddToViewport` _returnvalue 0)
  (`/Game/SunnyGame/Widgets/WBP_Fade.Fade Out` _returnvalue)
  (`KismetSystemLibrary.Delay` 4.0)
  (`GameplayStatics.OpenLevelBySoftObjectPtr` "/Game/SunnyGame/Maps/MainMenu.MainMenu"))

(fn `UserConstructionScript`)