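; BP_ProgressBase is a blocker, named as a base, that tells the player to defeat all enemies in the wave to progress.
; On BeginPlay it creates a WBP_Notifier widget and caches a BP_Sunny player reference.
; When BP_Sunny hits it, a DoOnce gate shows the message briefly, removes it and resets, preventing repeated triggers during display.
; It contains no wave-tracking or unblocking logic.
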(event `self.ReceiveBeginPlay`
  ; Reference notifier
  (bind _returnvalue (`|CreateWidget` "/Game/SunnyGame/Widgets/WBP_Notifier.WBP_Notifier_C"))
  (set `self.NotifierWidgetREF` _returnvalue)
  ; Reference Player
  (bind _asbp_sunny (cast `/Game/SunnyGame/Characters/Sunny/Blueprints/BP_Sunny` (`GameplayStatics.GetPlayerCharacter` 0)))
  (set `self.Reference Player` _asbp_sunny))

(event `self.ReceiveHit`
  (params (MyComp :type "PrimitiveComponent Object Reference") (Other :type "Actor Object Reference") (OtherComp :type "PrimitiveComponent Object Reference") (bSelfMoved :type Boolean) (HitLocation :type "Vector Structure") (HitNormal :type "Vector Structure") (NormalImpulse :type "Vector Structure") (Hit :type "HitResult Structure (by ref)"))
  ; Event Hit
  (cast `/Game/SunnyGame/Characters/Sunny/Blueprints/BP_Sunny` Other)
  (`/Engine/EditorBlueprintResources/StandardMacros.DoOnce` false :!label _label
    (:`Completed`
      (set `TextBlock.Text` "Defeat all enemies in this wave to progress" (`/Game/SunnyGame/Widgets/WBP_Notifier.Text_Narrative` (`self.NotifierWidgetREF`)))
      (`UserWidget.AddToViewport` (`self.NotifierWidgetREF`) 0)
      (`KismetSystemLibrary.Delay` 3.0)
      (`Widget.RemoveFromParent` (`self.NotifierWidgetREF`))
      (goto _label :!via `Reset`))))

(fn `UserConstructionScript`)