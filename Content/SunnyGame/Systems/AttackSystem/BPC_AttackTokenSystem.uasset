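; BPC_AttackTokenSystem is a Blueprint component that keeps a pool of attack tokens to gate attacks.
; ReserveAttackToken deducts the requested amount and returns true only when AttackTokenCount covers it, otherwise it returns false and leaves the pool untouched.
; ReturnAttackToken adds an amount back to the count, with no upper clamp or record of which caller holds tokens.
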(fn `Reserve Attack Token`
  (params (Amount :type Integer))
  (returns (`Success?` :type Boolean))
  ; Reserve Attack Tokens
  (if (>= (`self.Attack Token Count`) Amount)
    (set `self.Attack Token Count` (- (`self.Attack Token Count`) Amount))
    (return true)
    (else
      (return false))))

(fn `Return Attack Token`
  (params (Amount :type Integer))
  ; Return Token
  (set `self.Attack Token Count` (+ Amount (`self.Attack Token Count`))))