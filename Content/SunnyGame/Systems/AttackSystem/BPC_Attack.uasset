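; Actor component for melee combat that provides forward punch and kick hit detection plus an area-of-effect trace.
; Start events set looping timers by function name for each limb, sharing one handle that the End events clear.
; ForwardAttackTrace sphere-traces at an owner mesh socket, stopping the timer on hit, sending a damage message and spawning impact effects and sound.
; AOEAttackTrace multi-sphere-traces and only collects unique HitActors, without applying damage.
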(event `Start Right Punch Trace`
  ; Start Forward Attack Traces
  (bind _returnvalue (`KismetSystemLibrary.K2_SetTimer` null "Start Right Punch Trace " 0.0167 true))
  (set `self.Timer Handle` _returnvalue))

(event `Start Right Kick Trace`
  ; Start Forward Attack Traces
  (bind _returnvalue (`KismetSystemLibrary.K2_SetTimer` null "Start Right Kick Trace" 0.0167 true))
  (set `self.Timer Handle` _returnvalue))

(event `Start Left Punch Trace`
  ; Start Forward Attack Traces
  (bind _returnvalue (`KismetSystemLibrary.K2_SetTimer` null "Start Left Punch Trace" 0.0167 true))
  (set `self.Timer Handle` _returnvalue))

(event `Start Left Kick Trace`
  ; Start Forward Attack Traces
  (bind _returnvalue (`KismetSystemLibrary.K2_SetTimer` null "Start Left Kick Trace" 0.0167 true))
  (set `self.Timer Handle` _returnvalue))

(event `End Punch Trace`
  ; End Forward Attack Traces
  (`KismetSystemLibrary.K2_ClearAndInvalidateTimerHandle` (`self.Timer Handle`)))

(event `End Kick Trace`
  ; End Forward Attack Traces
  (`KismetSystemLibrary.K2_ClearAndInvalidateTimerHandle` (`self.Timer Handle`)))

(fn `AOE Attack Trace`
  (params (Start :type "Vector Structure") (End :type "Vector Structure") (Radius :type "Float (single-precision)") (`Damage Causer` :type "Actor Object Reference") (`Damage Amount` :type "Float (double-precision)"))
  (`KismetArrayLibrary.Array_Clear` (`self.Hit Actors`))
  (bind (_outhits _returnvalue) (`KismetSystemLibrary.SphereTraceMultiForObjects` Start End Radius (`|MakeArray` "ObjectTypeQuery3" "ObjectTypeQuery1" "ObjectTypeQuery4" "ObjectTypeQuery6" "ObjectTypeQuery2" :!type "EObjectTypeQuery Enum") false (`|MakeArray` (`self.GetOwner`))))
  (for _array_element _outhits
    (if _returnvalue
      (bind (_bblockinghit _binitialoverlap _time _distance _location _impactpoint _normal _impactnormal _physmat _hitactor) (`GameplayStatics.BreakHitResult` _array_element))
      (if (not (`KismetArrayLibrary.Array_Contains` (`self.Hit Actors`) _hitactor))
        (`KismetArrayLibrary.Array_AddUnique` (`self.Hit Actors`) _hitactor)))))

(fn `Forward Attack Trace`
  (params (`Damage Causer` :type "Actor Object Reference") (`Damage Amount` :type "Float (double-precision)") (`Socket Name` :type Name))
  (bind _returnvalue (`self.GetOwner`))
  (bind _returnvalue_2 (`SceneComponent.GetSocketLocation` (`Actor.GetComponentByClass` _returnvalue "/Script/Engine.MeshComponent") `Socket Name`))
  (bind (_outhit _returnvalue_3) (`KismetSystemLibrary.SphereTraceSingleForObjects` _returnvalue_2 _returnvalue_2 30.0 (`|MakeArray` "ObjectTypeQuery3" "ObjectTypeQuery1" "ObjectTypeQuery4" "ObjectTypeQuery6" "ObjectTypeQuery2" :!type "EObjectTypeQuery Enum") false (`|MakeArray` _returnvalue)))
  (if _returnvalue_3
    (`self.End Punch Trace`)
    (`self.End Kick Trace`)
    (bind (_bblockinghit _binitialoverlap _time _distance _location _impactpoint _normal _impactnormal _physmat _hitactor) (`GameplayStatics.BreakHitResult` _outhit))
    (message `/Game/SunnyGame/Systems/DamageSystem/BPI_DamagePlayer.Damage` _hitactor `Damage Amount` `Damage Causer`)
    (`NiagaraFunctionLibrary.SpawnSystemAtLocation` "/Game/SunnyGame/VFX/HitImpactFX/NS_HitImpact.NS_HitImpact" _location)
    (`GameplayStatics.PlaySoundAtLocation` "/Game/SunnyGame/Audio/HitImpacts/hit_impact_Cue.hit_impact_Cue" _location (struct) 1.0 1.0 0.0 null null null null)))