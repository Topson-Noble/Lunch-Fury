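; BP_HealthPack is a pickup that heals the player character BP_Sunny on overlap.
; On BeginPlay it sets its heal amount from the AI difficulty stored in BP_GameInstance, giving less health on harder settings.
; When Sunny enters its sphere, it calls Heal with that amount, spawns a Niagara heart effect at its location and destroys itself.
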(event `self.ReceiveBeginPlay`
  ; Switch 'Heal Amount' depending on difficulty
  (bind _asbp_game_instance (cast `/Game/SunnyGame/Systems/SaveSystem/BP_GameInstance` (`GameplayStatics.GetGameInstance`)))
  (switch `/Game/SunnyGame/Systems/AISystem/Enumerations/E_DifficultyState` (`/Game/SunnyGame/Systems/SaveSystem/BP_GameInstance.AI Difficulty` _asbp_game_instance)
    (:`NewEnumerator0`
      (set `self.Heal Amount` 100.0))
    (:`NewEnumerator1`
      (set `self.Heal Amount` 75.0))
    (:`NewEnumerator2`
      (set `self.Heal Amount` 50.0))))

(event `self.Sphere.OnComponentBeginOverlap`
  (params (OverlappedComponent :type "PrimitiveComponent Object Reference") (OtherActor :type "Actor Object Reference") (OtherComp :type "PrimitiveComponent Object Reference") (OtherBodyIndex :type Integer) (bFromSweep :type Boolean) (SweepResult :type "HitResult Structure (by ref)"))
  ; Heal Player
  (bind _asbp_sunny (cast `/Game/SunnyGame/Characters/Sunny/Blueprints/BP_Sunny` OtherActor))
  (`/Game/SunnyGame/Characters/Sunny/Blueprints/BP_Sunny.Heal` _asbp_sunny (`self.Heal Amount`))
  (`NiagaraFunctionLibrary.SpawnSystemAtLocation` "/Game/SunnyGame/VFX/BurstFX/NS_Heart.NS_Heart" (`self.K2_GetActorLocation`) (struct) (0.5 0.5 0.5))
  (`self.K2_DestroyActor`))

(fn `UserConstructionScript`)