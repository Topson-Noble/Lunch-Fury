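; Ninja enemy character that picks its behavior tree and damage from the game instance's AI difficulty.
; Punch and kick reserve an attack token on the target, then montage notifies fire socket-based traces through BPCAttack.
; Hits pause movement for a large (uppercut, roundkick) or small reaction, then set the AI attacking the damage causer.
; Death plays a moan and ragdolls the mesh; SetMovementSpeed just returns zero.
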(event `self.ReceiveBeginPlay`
  (`parent.ReceiveBeginPlay`)
  ; Set Behavior Tree depending on difficulty selected
  (bind _asbp_game_instance (cast `/Game/SunnyGame/Systems/SaveSystem/BP_GameInstance` (`GameplayStatics.GetGameInstance`)))
  (switch `/Game/SunnyGame/Systems/AISystem/Enumerations/E_DifficultyState` (`/Game/SunnyGame/Systems/SaveSystem/BP_GameInstance.AI Difficulty` _asbp_game_instance)
    (:`NewEnumerator0`
      (set `self.Behavior Tree` "/Game/SunnyGame/Systems/AISystem/BehaviorTrees/BT_EnemyNinjaEasy.BT_EnemyNinjaEasy")
      (set `self.Damage Amount` 12.0))
    (:`NewEnumerator1`
      (set `self.Behavior Tree` "/Game/SunnyGame/Systems/AISystem/BehaviorTrees/BT_EnemyNinjaMid.BT_EnemyNinjaMid")
      (set `self.Damage Amount` 20.0))
    (:`NewEnumerator2`
      (set `self.Behavior Tree` "/Game/SunnyGame/Systems/AISystem/BehaviorTrees/BT_EnemyNinjaHard.BT_EnemyNinjaHard")
      (set `self.Damage Amount` 30.0))))

(event `/Game/SunnyGame/Systems/DamageSystem/BPI_DamageEnemy.Damage Response`
  (params (`Damage Causer` :type "/Game/SunnyGame/Characters/Sunny/Blueprints/BP_Sunny Object Reference"))
  (bind _ai_controller_ref (`self.AI Controller REF`))
  (bind _ai_controller_ref_2 (`self.AI Controller REF`))
  ; Hit Reactions
  (`parent.Damage Response` `Damage Causer`)
  (`CharacterMovementComponent.DisableMovement` (`self.CharacterMovement`))
  (`GameplayStatics.PlaySoundAtLocation` "/Game/SunnyGame/Audio/MaleMoan/moan_Cue.moan_Cue" (`self.K2_GetActorLocation`) (struct) 1.0 1.0 0.0 null null null null)
  (if (`/Game/SunnyGame/Characters/Sunny/Blueprints/BP_Sunny.bIsUppercut?` `Damage Causer`)
    (`|PlayMontage` (`self.Mesh`) "/Game/SunnyGame/Characters/Enemies/Ninja/Animations/Montages/Standing_React_Large_From_Front_Montage.Standing_React_Large_From_Front_Montage" 1.0 0.1 :!label _label
      (:`OnCompleted`
        _)
      (:`OnInterrupted`
        _))
    (bind _output_get (set `/Game/SunnyGame/Systems/AISystem/BP_AIController.Attack Target` `Damage Causer` _ai_controller_ref_2))
    (`/Game/SunnyGame/Systems/AISystem/BP_AIController.Set State As Attacking` _ai_controller_ref_2 _output_get)
    (`CharacterMovementComponent.SetMovementMode` (`self.CharacterMovement`) "MOVE_Walking" 0)
    (elif (`/Game/SunnyGame/Characters/Sunny/Blueprints/BP_Sunny.bIsRoundKick?` `Damage Causer`)
      (goto _label)
      (else
        (`|PlayMontage` (`self.Mesh`) "/Game/SunnyGame/Characters/Enemies/Ninja/Animations/Montages/Standing_React_Small_From_Front_02_Montage.Standing_React_Small_From_Front_02_Montage" 1.2
          (:`OnCompleted`
            _)
          (:`OnInterrupted`
            _))
        (bind _output_get_2 (set `/Game/SunnyGame/Systems/AISystem/BP_AIController.Attack Target` `Damage Causer` _ai_controller_ref))
        (`/Game/SunnyGame/Systems/AISystem/BP_AIController.Set State As Attacking` _ai_controller_ref _output_get_2)
        (`CharacterMovementComponent.SetMovementMode` (`self.CharacterMovement`) "MOVE_Walking" 0)))))

(event `/Game/SunnyGame/Systems/DamageSystem/BPI_DamageEnemy.Death`
  ; Death Logic
  (`parent.Death`)
  (`GameplayStatics.PlaySoundAtLocation` "/Game/SunnyGame/Audio/MaleMoan/death_moan_Cue.death_moan_Cue" (`self.K2_GetActorLocation`) (struct) 1.0 1.0 0.0 null null null null)
  (`PrimitiveComponent.SetSimulatePhysics` (`self.Mesh`) true))

(event `self.Punch Attack`
  (params (`Attack Target` :type "Actor Object Reference"))
  ; Punch and Kick Attacks
  (`parent.Punch Attack` `Attack Target`)
  (bind _success_ (message `/Game/SunnyGame/Systems/AttackSystem/BPI_AttackToken.Reserve Attack Token` `Attack Target` 1))
  (if _success_
    (bind _notifyname (`|PlayMontage` (`self.Mesh`) "/Game/SunnyGame/Characters/Enemies/Ninja/Animations/Montages/Cross_Punch_Montage.Cross_Punch_Montage" 2.0)
      (:`OnCompleted`
        (`self.OnPunchAttackEnd` :!label _label_2)
        (message `/Game/SunnyGame/Systems/AttackSystem/BPI_AttackToken.Return Attack Token` `Attack Target` 1))
      (:`OnInterrupted`
        (goto _label_2))
      (:`OnNotifyBegin`
        (if (== _notifyname "DoAttackTrace")
          (`/Game/SunnyGame/Systems/AttackSystem/BPC_Attack.Forward Attack Trace` (`self.BPC_Attack`) self (`self.Damage Amount`) "R Hand Socket")
          (`RadialForceComponent.FireImpulse` (`self.RadialForce`)))))
    (else
      (`KismetSystemLibrary.DelayUntilNextTick`)
      (`self.OnPunchAttackEnd`))))

(event `self.Kick Attack`
  (params (`Attack Target` :type "Actor Object Reference"))
  ; Punch and Kick Attacks
  (`parent.Kick Attack` `Attack Target`)
  (bind _success_ (message `/Game/SunnyGame/Systems/AttackSystem/BPI_AttackToken.Reserve Attack Token` `Attack Target` 1))
  (if _success_
    (bind _notifyname (`|PlayMontage` (`self.Mesh`) "/Game/SunnyGame/Characters/Enemies/Ninja/Animations/Montages/Side_Kick_Montage.Side_Kick_Montage" 2.0)
      (:`OnCompleted`
        (`self.OnKickAttackEnd` :!label _label_3)
        (message `/Game/SunnyGame/Systems/AttackSystem/BPI_AttackToken.Return Attack Token` `Attack Target` 1))
      (:`OnInterrupted`
        (goto _label_3))
      (:`OnNotifyBegin`
        (if (== _notifyname "DoKickTrace")
          (`/Game/SunnyGame/Systems/AttackSystem/BPC_Attack.Forward Attack Trace` (`self.BPC_Attack`) self (`self.Damage Amount`) "R Foot Socket"))))
    (else
      (`KismetSystemLibrary.DelayUntilNextTick`)
      (`self.OnPunchAttackEnd`))))

(fn `Set Movement Speed`
  (params (`Movement Types` :type "/Game/SunnyGame/Systems/AISystem/Enumerations/E_MovementSpeed Enum" :default "NewEnumerator0"))
  (returns (Speed :type "Float (double-precision)"))
  (return 0.0))

(fn `UserConstructionScript`
  (`parent.UserConstructionScript`))