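; Base enemy character that provides health, death and AI-facing combat queries, with empty punch and kick attack events for combat.
; Damage updates a floating health bar, flashes an overlay material and switches the AI controller to its taking-damage state.
; Death stops AI logic, collision and movement, returns the attack token to the blackboard target, then destroys the actor after a delay.
; Also exposes team, range, speed and its own attack-token component.
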(event `self.ReceiveBeginPlay`
  ; Reference AI Controller
  (bind _asbp_aicontroller (cast `/Game/SunnyGame/Systems/AISystem/BP_AIController` (`AIBlueprintHelperLibrary.GetAIController` self)))
  (set `self.AI Controller REF` _asbp_aicontroller)
  ; Add Health Bar
  (bind _returnvalue (`|CreateWidget` "/Game/SunnyGame/Widgets/WBP_FloatingHealthBar.WBP_FloatingHealthBar_C"))
  (set `self.HealthBarWidget REF` _returnvalue)
  (set `/Game/SunnyGame/Widgets/WBP_FloatingHealthBar.Current Health` (`self.Current Health`) (`self.HealthBarWidget REF`))
  (set `/Game/SunnyGame/Widgets/WBP_FloatingHealthBar.Max Health` (`self.Max Health`) (`self.HealthBarWidget REF`))
  (`WidgetComponent.SetWidget` (`self.Health Bar Component`) (`self.HealthBarWidget REF`)))

(event `/Game/SunnyGame/Systems/DamageSystem/BPI_DamageEnemy.Damage`
  (params (`Damage Amount` :type "Float (double-precision)") (`Damage Causer` :type "/Game/SunnyGame/Characters/Sunny/Blueprints/BP_Sunny Object Reference"))
  ; Health System - Taking Damage
  (if (not (`self.bIsDead?`))
    (bind _output_get (set `self.Current Health` (`KismetMathLibrary.FClamp` (- (`self.Current Health`) `Damage Amount`) 0.0 (`self.Max Health`))))
    (set `/Game/SunnyGame/Widgets/WBP_FloatingHealthBar.Current Health` _output_get (`self.HealthBarWidget REF`))
    (`/Game/SunnyGame/Systems/DamageSystem/BPI_DamageEnemy.Damage Response` `Damage Causer`)
    (if (<= (`self.Current Health`) 0.0)
      (set `self.bIsDead?` true)
      (`/Game/SunnyGame/Systems/DamageSystem/BPI_DamageEnemy.Death`))))

(event `/Game/SunnyGame/Systems/DamageSystem/BPI_DamageEnemy.Damage Response`
  (params (`Damage Causer` :type "/Game/SunnyGame/Characters/Sunny/Blueprints/BP_Sunny Object Reference"))
  ; Damage Response
  (`self.Hit Flash`)
  (`/Game/SunnyGame/Systems/AISystem/BP_AIController.Set State As Taking Damage` (`self.AI Controller REF`)))

(event `/Game/SunnyGame/Systems/DamageSystem/BPI_DamageEnemy.Death`
  ; Death Logic
  (`ActorComponent.K2_DestroyComponent` (`self.Health Bar Component`))
  (`PrimitiveComponent.SetCollisionEnabled` (`self.CapsuleComponent`) "NoCollision")
  (`CharacterMovementComponent.DisableMovement` (`self.CharacterMovement`))
  (`BrainComponent.StopLogic` (`AIController.BrainComponent` (`self.AI Controller REF`)) "Dead")
  (message `/Game/SunnyGame/Systems/AttackSystem/BPI_AttackToken.Return Attack Token` (`BlackboardComponent.GetValueAsObject` (`AIController.Blackboard` (`self.AI Controller REF`)) (`self.Attack Target Key`)) 1)
  (`self.OnDeath`)
  (`KismetSystemLibrary.Delay` 4.0)
  (`self.K2_DestroyActor`))

(event `Hit Flash`
  ; Hit Flash
  (`MeshComponent.SetOverlayMaterial` (`self.Mesh`) "/Game/SunnyGame/Materials/M_HitFlash.M_HitFlash")
  (`KismetSystemLibrary.Delay` 0.1)
  (`MeshComponent.SetOverlayMaterial` (`self.Mesh`) null))

(event `Punch Attack`
  (params (`Attack Target` :type "Actor Object Reference"))
  ; Attack
)

(event `Kick Attack`
  (params (`Attack Target` :type "Actor Object Reference"))
  ; Attack
)

(event `/Game/SunnyGame/Systems/AttackSystem/BPI_AttackToken.Return Attack Token`
  (params (`Token Amount` :type Integer))
  ; Return Attack Token
  (`/Game/SunnyGame/Systems/AttackSystem/BPC_AttackTokenSystem.Return Attack Token` (`self.BPC_AttackTokenSystem`) `Token Amount`))

(fn `Check Is Dead`
  (returns (`bIsDead?` :type Boolean))
  ; Check is Dead
  (return (`self.bIsDead?`)))

(fn `Get Ideal Range`
  (returns (`Attack Distance` :type "Float (double-precision)") (`Defend Distance` :type "Float (double-precision)"))
  (return 100.0 500.0))

(fn `Get Team Number`
  (returns (`Team Number` :type Integer))
  ; Get Team Number
  (return (`self.Team Number`)))

(fn `Reserve Attack Token`
  (params (Amount :type Integer))
  (returns (`Success?` :type Boolean))
  (bind _success_ (`/Game/SunnyGame/Systems/AttackSystem/BPC_AttackTokenSystem.Reserve Attack Token` (`self.BPC_AttackTokenSystem`) Amount))
  (return _success_))

(fn `Set Movement Speed`
  (params (`Movement Types` :type "/Game/SunnyGame/Systems/AISystem/Enumerations/E_MovementSpeed Enum" :default "NewEnumerator0"))
  (returns (Speed :type "Float (double-precision)"))
  ; Movement Speed
  (bind _output_get (set `CharacterMovementComponent.MaxWalkSpeed` (select `/Game/SunnyGame/Systems/AISystem/Enumerations/E_MovementSpeed` `Movement Types` :`NewEnumerator1` 150.0 :`NewEnumerator2` 300.0 :!type "Float (single-precision)") (`self.CharacterMovement`)))
  (return _output_get))

(fn `UserConstructionScript`)