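; BP_LunchBox is an end-of-game pickup that becomes available once the player's final wave is cleared.
; Tick polls BP_Sunny's IsFinalWaveCleared and, through a DoOnce, plays a sound and unhides the actor.
; Trigger box overlaps show the prompt widget only after that clear and hide it on exit.
; Interact sets EndGame on the player, plays a sound and destroys the lunchbox after a brief delay.
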(event `self.ReceiveBeginPlay`
  ; Reference Player
  (bind _asbp_sunny (cast `/Game/SunnyGame/Characters/Sunny/Blueprints/BP_Sunny` (`GameplayStatics.GetPlayerCharacter` 0)))
  (set `self.Player REF` _asbp_sunny))

(event `self.Trigger Box.OnComponentBeginOverlap`
  (params (OverlappedComponent :type "PrimitiveComponent Object Reference") (OtherActor :type "Actor Object Reference") (OtherComp :type "PrimitiveComponent Object Reference") (OtherBodyIndex :type Integer) (bFromSweep :type Boolean) (SweepResult :type "HitResult Structure (by ref)"))
  ; Show and Hide Prompts
  (bind _asbp_sunny (cast `/Game/SunnyGame/Characters/Sunny/Blueprints/BP_Sunny` OtherActor))
  (if (`/Game/SunnyGame/Characters/Sunny/Blueprints/BP_Sunny.bIsFinalWaveCleared?` _asbp_sunny)
    (`SceneComponent.SetVisibility` (`self.Widget`) true false)))

(event `self.Trigger Box.OnComponentEndOverlap`
  (params (OverlappedComponent :type "PrimitiveComponent Object Reference") (OtherActor :type "Actor Object Reference") (OtherComp :type "PrimitiveComponent Object Reference") (OtherBodyIndex :type Integer))
  ; Show and Hide Prompts
  (cast `/Game/SunnyGame/Characters/Sunny/Blueprints/BP_Sunny` OtherActor)
  (`SceneComponent.SetVisibility` (`self.Widget`) false false))

(event `/Game/SunnyGame/Systems/InteractionSystem/BPI_Interact.Interact`
  ; Pickup Lunchbox
  (set `/Game/SunnyGame/Characters/Sunny/Blueprints/BP_Sunny.bEndGame?` true (`self.Player REF`))
  (`GameplayStatics.PlaySound2D` "/Engine/VREditor/Sounds/UI/Dockable_Window_Open.Dockable_Window_Open" 1.0 1.0 0.0 null null)
  (`KismetSystemLibrary.Delay` 0.1)
  (`self.K2_DestroyActor`))

(event `self.ReceiveTick`
  (params (DeltaSeconds :type "Float (single-precision)"))
  ; Constantly check if final wave is cleared
  (if (`/Game/SunnyGame/Characters/Sunny/Blueprints/BP_Sunny.bIsFinalWaveCleared?` (`self.Player REF`))
    (`/Engine/EditorBlueprintResources/StandardMacros.DoOnce` false
      (:`Completed`
        (`GameplayStatics.PlaySound2D` "/Engine/VREditor/Sounds/UI/Dockable_Window_Close.Dockable_Window_Close" 1.0 1.0 0.0 null null)
        (`self.SetActorHiddenInGame` false)))))

(fn `UserConstructionScript`)